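; BP_enemy is an enemy Blueprint with a flipbook sprite and a networked moving-or-idle state.
; MovementState forwards the flag to a server event that sets IsMoving, which has an OnRep handler.
; That handler branches on IsMoving, but its idle and walk flipbook calls, fed from EnemyInfo, are unwired and never run.
; GetEnemyRef returns the enemy itself.
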(event `/Game/enemy2/Blueprints/INT_EnemyBae.MovementState`
  (params (IsMoving :type Boolean))
  (`self.SRV_MovementState` IsMoving))

(event `SRV_MovementState`
  (params (IsMoving :type Boolean))
  (set `self.IsMoving` IsMoving))

(fn `GetEnemyRef`
  (returns (enemy :type "/Game/Assets/enemy2/Blueprints/BP_enemy Object Reference"))
  (return self))

(fn `OnRep_IsMoving`
  (if (not (`self.IsMoving`))
    _))

(fn `UserConstructionScript`)