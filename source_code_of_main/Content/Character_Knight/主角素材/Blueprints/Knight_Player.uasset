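; Player-controlled Paper2D knight character for a side-scrolling platformer, with Enhanced Input for jumping and moving along X.
; Each tick picks idle, run, jump or fall flipbooks from movement state and turns control rotation to face horizontal velocity.
; Background sprites under Bg get dynamic materials with per-layer parallax multipliers, fed the camera's X position every frame.
; An unused-looking CustomEvent duplicates the animation logic in UpdateAnimation.
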(event `self.ReceiveBeginPlay`
  (`self.Init Input`)
  (`ActorComponent.SetIsReplicated` (`self.Sprite`) true)
  ;[1 1 1] Init dynamic material
  (for (_array_element _array_index) (`SceneComponent.GetChildrenComponents` (`self.bg`) false)
    (bind `_aspaper_sprite组件` (cast `PaperSpriteComponent` _array_element))
    (bind _returnvalue (`PrimitiveComponent.CreateDynamicMaterialInstance` `_aspaper_sprite组件` 0 null "None"))
    (`KismetArrayLibrary.Array_Add` (`self.dynamic layers`) _returnvalue)
    (`MaterialInstanceDynamic.SetScalarParameterValue` _returnvalue "ParallaxMultiplier" (`|GetArrayItem` (`self.parallaxmultiplier`) _array_index))))

(event `self.ReceiveTick`
  (params (DeltaSeconds :type "Float (single-precision)"))
  (bind _returnvalue_x (`KismetMathLibrary.BreakVector` (`SceneComponent.K2_GetComponentLocation` (`self.Camera`))))
  ;[0.05098 0.05098 0.05098] Animation and Rotation will update every frame
  (`self.UpdateAnimation`)
  (`self.SetControllerRotation`)
  (for _array_element (`self.dynamic layers`)
    (`MaterialInstanceDynamic.SetScalarParameterValue` _array_element "CameraPosX" _returnvalue_x)))

(event `EnhancedInput|/Game/Character_Knight/主角素材/Input/Actions/IA_Jump`
  (params (ActionValue :type Boolean) (ElapsedSeconds :type "Float (double-precision)") (TriggeredSeconds :type "Float (double-precision)") (InputAction :type "InputAction Object Reference" :default "/Game/Character_Knight/主角素材/Input/Actions/IA_Jump.IA_Jump"))
  (:`Started`
    (`self.Jump`))
  (:`Completed`
    (`self.StopJumping`)))

(event `EnhancedInput|/Game/Character_Knight/主角素材/Input/Actions/IA_Move`
  (params (ActionValue :type "Float (double-precision)") (ElapsedSeconds :type "Float (double-precision)") (TriggeredSeconds :type "Float (double-precision)") (InputAction :type "InputAction Object Reference" :default "/Game/Character_Knight/主角素材/Input/Actions/IA_Move.IA_Move"))
  (:`Triggered`
    (`self.AddMovementInput` (1.0 0.0 0.0) ActionValue)
    (`Controller.SetControlRotation` (`self.GetController`) (select `bool` (> ActionValue 0.0) :`false` (`KismetMathLibrary.MakeRotator` 0.0 0.0 180.0) :`true` (`KismetMathLibrary.MakeRotator` 0.0)))))

(event `CustomEvent`
  (bind (_returnvalue_x _returnvalue_y _returnvalue_z) (`KismetMathLibrary.BreakVector` (`self.GetVelocity`)))
  (if (`NavMovementComponent.IsMovingOnGround` (`self.CharacterMovement`))
    (if (> (`KismetMathLibrary.VSize` (`self.GetVelocity`)) 0.0)
      (`PaperFlipbookComponent.SetFlipbook` (`self.Sprite`) "/Game/Character_Knight/主角素材/Flipbooks/RUN/Running_flipbook.Running_flipbook")
      (else
        (`PaperFlipbookComponent.SetFlipbook` (`self.Sprite`) "/Game/Character_Knight/主角素材/Flipbooks/IDLE/Idle_flipbook.Idle_flipbook")))
    (elif (< _returnvalue_z -100.0)
      (`PaperFlipbookComponent.SetFlipbook` (`self.Sprite`) "/Game/Character_Knight/主角素材/Flipbooks/JUMP/Fall_flipbook.Fall_flipbook")
      (else
        (`PaperFlipbookComponent.SetFlipbook` (`self.Sprite`) "/Game/Character_Knight/主角素材/Flipbooks/JUMP/Jumping_flipbook.Jumping_flipbook")))))

(event `SetControllerRotation`
  (bind _returnvalue (`self.GetController`))
  (bind _returnvalue_2 (`self.GetController`))
  ;[0.05098 0.05098 0.05098] Turns controller left or right depending on velocity
  (`/Engine/EditorBlueprintResources/StandardMacros.CompareFloat` (.x (`self.GetVelocity`))
    (:`>`
      (`/Engine/EditorBlueprintResources/StandardMacros.IsValid` _returnvalue_2
        (:`Is Valid`
          (`Controller.SetControlRotation` _returnvalue_2 (`KismetMathLibrary.MakeRotator` 0.0)))))
    (:`<`
      (`/Engine/EditorBlueprintResources/StandardMacros.IsValid` _returnvalue
        (:`Is Valid`
          (`Controller.SetControlRotation` _returnvalue (`KismetMathLibrary.MakeRotator` 0.0 0.0 180.0)))))))

(fn `Init Input`
  (bind `_as玩家控制器` (cast `PlayerController` (`self.GetController`)))
  (`EnhancedInputSubsystemInterface.AddMappingContext` (pcsubsystem `EnhancedInputLocalPlayerSubsystem` `_as玩家控制器`) "/Game/Character_Knight/主角素材/Input/IMC_Platforming.IMC_Platforming" 0 (struct)))

(fn `UpdateAnimation`
  (bind (_returnvalue_x _returnvalue_y _returnvalue_z) (`KismetMathLibrary.BreakVector` (`self.GetVelocity`)))
  (if (`NavMovementComponent.IsMovingOnGround` (`self.CharacterMovement`))
    (if (> (`KismetMathLibrary.VSize` (`self.GetVelocity`)) 0.0)
      (`PaperFlipbookComponent.SetFlipbook` (`self.Sprite`) "/Game/Character_Knight/主角素材/Flipbooks/RUN/Running_flipbook.Running_flipbook")
      (else
        (`PaperFlipbookComponent.SetFlipbook` (`self.Sprite`) "/Game/Character_Knight/主角素材/Flipbooks/IDLE/Idle_flipbook.Idle_flipbook")))
    (elif (< _returnvalue_z -100.0)
      (`PaperFlipbookComponent.SetFlipbook` (`self.Sprite`) "/Game/Character_Knight/主角素材/Flipbooks/JUMP/Fall_flipbook.Fall_flipbook")
      (else
        (`PaperFlipbookComponent.SetFlipbook` (`self.Sprite`) "/Game/Character_Knight/主角素材/Flipbooks/JUMP/Jumping_flipbook.Jumping_flipbook")))))

(fn `UserConstructionScript`)